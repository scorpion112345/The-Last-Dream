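; A floor button actor that opens a pair of doors when something overlaps its trigger box.
; On BeginPlay it caches each door's starting rotation and a target yawed 90 degrees in opposite directions.
; The first overlap, gated by DoOnce, swaps the button mesh to an active material and plays two timelines that lerp each door toward its target rotation.
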(event OnComponentBeginOverlap(Box)
  (params (OverlappedComponent :type Primitive%20Component%20Object%20Reference) (OtherActor :type Actor%20Object%20Reference) (OtherComp :type Primitive%20Component%20Object%20Reference) (OtherBodyIndex :type Integer) (bFromSweep :type Boolean) (SweepResult :type Hit%20Result%20Structure%20%28by%20ref%29))
  (Utilities|FlowControl|DoOnce false
    (:Completed
      (Rendering|Material|SetMaterial (Variables|Default|GetStaticMesh) 0 "/Game/AfterTheDream/Assets/Materials/M_Tile_Boton_Active.M_Tile_Boton_Active")
      (Utilities|FlowControl|Sequence
        (:then_0
          (bind _newtrack_0 (Timeline|Timeline_0 Play)
            (:Update
              (Transformation|SetActorRotation (Variables|Default|GetPuerta) (Math|Rotator|Lerp(Rotator) (Variables|Default|GetP_Detecha_Inicial) (Variables|Default|GetP_Derecha_Final) _newtrack_0)))))
        (:then_1
          (bind _newtrack_0_2 (Timeline|Timeline_1 Play)
            (:Update
              (Transformation|SetActorRotation (Variables|Default|GetPuerta2) (Math|Rotator|Lerp(Rotator) (Variables|Default|GetP_Izquierda_Inicial) (Variables|Default|GetP_Izquierda_Final) _newtrack_0_2)))))))))

(event EventBeginPlay
  (bind _puerta (Variables|Default|GetPuerta))
  (bind _puerta2 (Variables|Default|GetPuerta2))
  (bind _returnvalue (Transformation|GetActorRotation _puerta2))
  (bind _returnvalue_2 (Transformation|GetActorRotation _puerta))
  (bind (_roll _pitch _yaw) (Math|Rotator|BreakRotator _returnvalue))
  (bind (_roll_2 _pitch_2 _yaw_2) (Math|Rotator|BreakRotator _returnvalue_2))
  (Utilities|FlowControl|Sequence
    (:then_0
      (Variables|Default|SetP_Detecha_Inicial _returnvalue_2)
      (Variables|Default|SetP_Derecha_Final (Math|Rotator|MakeRotator _roll_2 _pitch_2 (+ _yaw_2 9e+01)))
      (Variables|Default|SetP_Izquierda_Inicial _returnvalue)
      (Variables|Default|SetP_Izquierda_Final (Math|Rotator|MakeRotator _roll _pitch (+ _yaw -9e+01))))))

(fn ConstructionScript)